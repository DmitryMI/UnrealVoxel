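; Player controller for the dynamic geometry voxel test level, highlighting the voxel the player looks at.
; On BeginPlay it caches the level's VoxelWorld actor and adds the dynamic geometry HUD widget to the viewport.
; Each tick it runs a filtered voxel line trace from the view point and draws a blue debug box around the hit voxel, sized to the world's voxel size.
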(event `self.ReceiveBeginPlay`
  (bind _returnvalue (`GameplayStatics.GetActorOfClass` "/Script/VoxelEngine.VoxelWorld"))
  (set `self.VoxelWorld` _returnvalue)
  (bind _returnvalue_2 (`|CreateWidget` "/Game/VoxelEngine/Levels/DynamicGeometryTest/WB_DynamicGeometryHud.WB_DynamicGeometryHud_C"))
  (`UserWidget.AddToViewport` _returnvalue_2 0))

(event `self.ReceiveTick`
  (params (DeltaSeconds :type "Float (single-precision)"))
  (bind (_location _rotation) (`self.GetPlayerViewPoint`))
  (bind _tracelength (`self.TraceLength`))
  (bind _voxelworld (`self.VoxelWorld`))
  (bind _returnvalue (/ (`VoxelWorld.GetVoxelSizeWorld` _voxelworld) 2.0))
  (bind (_outhitcoord _returnvalue_2) (`VoxelQueryUtils.VoxelLineTraceFilterSingle` (`self.VoxelWorld`) _location (* (`KismetMathLibrary.Conv_RotatorToVector` _rotation) (`KismetMathLibrary.MakeVector` _tracelength _tracelength _tracelength)) (make `VoxelLineTraceFilterParams` "Negative" "Negative" (`self.TraceLength`))))
  (if _returnvalue_2
    (`KismetSystemLibrary.DrawDebugBox` (`VoxelWorld.GetVoxelCenterWorld` _voxelworld _outhitcoord) (`KismetMathLibrary.MakeVector` _returnvalue _returnvalue _returnvalue) (struct :`G` 0.000169 :`B` 1.0 :`A` 1.0) (struct) 0.0 4.0)))

(fn `UserConstructionScript`)