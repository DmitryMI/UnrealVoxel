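; Test player controller for voxel terrain collision that finds the voxel in the center of the player's view.
; BeginPlay caches the VoxelWorld, adds the test HUD and installs the terrain collision input mapping.
; Each tick, a filtered voxel line trace from the view point stores the hit coordinate, outlines that voxel with a debug box and prints it.
; The hit flag is only set on success, never cleared on a miss.
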(event `self.ReceiveBeginPlay`
  (bind _returnvalue (`GameplayStatics.GetActorOfClass` "/Script/VoxelEngine.VoxelWorld"))
  (set `self.VoxelWorld` _returnvalue)
  (bind _returnvalue_2 (`|CreateWidget` "/Game/VoxelEngine/Test/TerrainCollisionTest/WB_TerrainCollisionHud.WB_TerrainCollisionHud_C"))
  (`UserWidget.AddToViewport` _returnvalue_2 0)
  (`EnhancedInputSubsystemInterface.AddMappingContext` (subsystem `EnhancedInputLocalPlayerSubsystem`) "/Game/VoxelEngine/Test/TerrainCollisionTest/IMC_TerrainCollision.IMC_TerrainCollision" 0 (struct)))

(event `self.ReceiveTick`
  (params (DeltaSeconds :type "Float (single-precision)"))
  (`self.FindBlockUnderCursor`))

(fn `FindBlockUnderCursor`
  (bind (_location _rotation) (`self.GetPlayerViewPoint`))
  (bind _tracelength (`self.TraceLength`))
  (bind _voxelworld (`self.VoxelWorld`))
  (bind _returnvalue (/ (`VoxelWorld.GetVoxelSizeWorld` _voxelworld) 2.0))
  (bind (_outhitcoord _returnvalue_2) (`VoxelQueryUtils.VoxelLineTraceFilterSingle` (`self.VoxelWorld`) _location (* (`KismetMathLibrary.Conv_RotatorToVector` _rotation) (`KismetMathLibrary.MakeVector` _tracelength _tracelength _tracelength)) (make `VoxelLineTraceFilterParams` (`self.TraceLength`) true "Negative" "Negative")))
  (if _returnvalue_2
    (bind _output_get (set `self.VoxelUnderCursor` _outhitcoord))
    (set `self.HasVoxelUnderCursor` _returnvalue_2)
    (`KismetSystemLibrary.DrawDebugBox` (`VoxelWorld.GetVoxelCenterWorld` _voxelworld _outhitcoord) (`KismetMathLibrary.MakeVector` _returnvalue _returnvalue _returnvalue) (struct :`G` 0.000169 :`B` 1.0 :`A` 1.0) (struct) 0.0 4.0)
    (`KismetSystemLibrary.PrintString` (`KismetStringLibrary.Conv_IntVectorToString` _output_get) true false (struct :`G` 0.66 :`B` 1.0 :`A` 1.0) 0.0)))

(fn `UserConstructionScript`)