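; Test player controller for the voxel engine that tracks the voxel under the view ray and the adjacent cell where a block would be placed.
; BeginPlay caches the VoxelWorld, adds the JSON persistence HUD and registers the block placer input mapping.
; Each Tick runs a filtered voxel line trace, stores both coordinates and optionally draws debug boxes.
; No placement or input handling appears in these graphs.
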(event `self.ReceiveBeginPlay`
  (bind _returnvalue (`GameplayStatics.GetActorOfClass` "/Script/VoxelEngine.VoxelWorld"))
  (set `self.VoxelWorld` _returnvalue)
  (bind _returnvalue_2 (`|CreateWidget` "/Game/VoxelEngine/Test/Blueprints/WB_JsonPersistenceHud.WB_JsonPersistenceHud_C"))
  (`UserWidget.AddToViewport` _returnvalue_2 0)
  (`EnhancedInputSubsystemInterface.AddMappingContext` (subsystem `EnhancedInputLocalPlayerSubsystem`) "/Game/VoxelEngine/Test/Input/IMC_BlockPlacer.IMC_BlockPlacer" 0 (struct)))

(event `self.ReceiveTick`
  (params (DeltaSeconds :type "Float (single-precision)"))
  (`self.FindBlockUnderCursor`))

(fn `FindBlockUnderCursor`
  (bind (_location _rotation) (`self.GetPlayerViewPoint`))
  (bind _tracelength (`self.TraceLength`))
  (bind _voxelworld (`self.VoxelWorld`))
  (bind _returnvalue (* (`KismetMathLibrary.Conv_RotatorToVector` _rotation) (`KismetMathLibrary.MakeVector` _tracelength _tracelength _tracelength)))
  (bind _returnvalue_2 (/ (`VoxelWorld.GetVoxelSizeWorld` _voxelworld) 2.0))
  (bind (_outhitcoord _returnvalue_3) (`VoxelQueryUtils.VoxelLineTraceFilterSingle` (`self.VoxelWorld`) _location _returnvalue (make `VoxelLineTraceFilterParams` (`self.TraceLength`) true "Negative" "Negative")))
  (set `self.HasVoxelUnderCursor` _returnvalue_3)
  (if _returnvalue_3
    (bind _output_get (set `self.VoxelUnderCursor` _outhitcoord))
    (bind _output_get_2 (set `self.HasVoxelUnderCursor` _returnvalue_3))
    (if _output_get_2
      (bind (_outadjacentvoxel _returnvalue_4) (`VoxelQueryUtils.GetLookedThroughAdjacentVoxel` (`self.VoxelWorld`) _output_get _location _returnvalue))
      (if _returnvalue_4
        (bind _output_get_3 (set `self.PlaceVoxelCoord` _outadjacentvoxel))
        (if (`self.DebugDrawVoxelUnderCursor`)
          (`KismetSystemLibrary.DrawDebugBox` (`VoxelWorld.GetVoxelCenterWorld` _voxelworld _outhitcoord) (`KismetMathLibrary.MakeVector` _returnvalue_2 _returnvalue_2 _returnvalue_2) (struct :`G` 0.000169 :`B` 1.0 :`A` 1.0) (struct) 0.0 4.0))
        (`KismetSystemLibrary.PrintString` (`KismetStringLibrary.Conv_IntVectorToString` _output_get) true false (struct :`G` 0.66 :`B` 1.0 :`A` 1.0) 0.0)
        (if (`self.DebugDrawPlaceVoxel`)
          (bind _returnvalue_5 (`VoxelWorld.GetVoxelBoundingBox` (`self.VoxelWorld`) _output_get_3))
          (`KismetSystemLibrary.DrawDebugBox` (`KismetMathLibrary.GetBoxCenter` _returnvalue_5) (/ (`KismetMathLibrary.GetBoxSize` _returnvalue_5) (2.0 2.0 2.0)) (struct :`R` 0.144702 :`G` 1.0 :`A` 1.0) (struct) 0.0 4.0))))))

(fn `UserConstructionScript`)