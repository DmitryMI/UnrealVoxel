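; Test pawn that lets the player place and destroy blocks in the voxel world through Enhanced Input actions.
; Each action reads the targeted coordinates and hover flag from BP_BlockPlacerPlayerController, then calls ChangeVoxel on its VoxelWorld with a hardcoded type to place or clear a voxel.
; On-screen prints report whether each change succeeded or failed.
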(event `self.ReceiveBeginPlay`)

(event `EnhancedInput|/Game/VoxelEngine/Test/Input/IA_PlaceVoxel`
  (params (ActionValue :type Boolean) (ElapsedSeconds :type "Float (double-precision)") (TriggeredSeconds :type "Float (double-precision)") (InputAction :type "InputAction Object Reference" :default "/Game/VoxelEngine/Test/Input/IA_PlaceVoxel.IA_PlaceVoxel"))
  (bind _returnvalue (`self.GetController`))
  (:`Triggered`
    (`/Engine/EditorBlueprintResources/StandardMacros.IsValid` _returnvalue
      (:`Is Valid`
        (bind _asbp_navigation_player_controller (cast `/Game/VoxelEngine/Test/Blueprints/BP_BlockPlacerPlayerController` _returnvalue))
        (if (`/Game/VoxelEngine/Test/Blueprints/BP_BlockPlacerPlayerController.HasVoxelUnderCursor` _asbp_navigation_player_controller)
          (bind _returnvalue_2 (`VoxelWorld.ChangeVoxel` (`/Game/VoxelEngine/Test/Blueprints/BP_BlockPlacerPlayerController.VoxelWorld` _asbp_navigation_player_controller) (`/Game/VoxelEngine/Test/Blueprints/BP_BlockPlacerPlayerController.PlaceVoxelCoord` _asbp_navigation_player_controller) 3))
          (if (`|EnumEquality` _returnvalue_2 "Executed")
            (`KismetSystemLibrary.PrintString` "Voxel placed")
            (else
              (`KismetSystemLibrary.PrintString` "Failed to place voxel" true true (struct :`R` 1.0 :`G` 0.009094 :`A` 1.0)))))))))

(event `EnhancedInput|/Game/VoxelEngine/Test/Input/IA_DestroyVoxel`
  (params (ActionValue :type Boolean) (ElapsedSeconds :type "Float (double-precision)") (TriggeredSeconds :type "Float (double-precision)") (InputAction :type "InputAction Object Reference" :default "/Game/VoxelEngine/Test/Input/IA_DestroyVoxel.IA_DestroyVoxel"))
  (bind _returnvalue (`self.GetController`))
  (:`Triggered`
    (`/Engine/EditorBlueprintResources/StandardMacros.IsValid` _returnvalue
      (:`Is Valid`
        (bind _asbp_navigation_player_controller (cast `/Game/VoxelEngine/Test/Blueprints/BP_BlockPlacerPlayerController` _returnvalue))
        (if (`/Game/VoxelEngine/Test/Blueprints/BP_BlockPlacerPlayerController.HasVoxelUnderCursor` _asbp_navigation_player_controller)
          (bind _returnvalue_2 (`VoxelWorld.ChangeVoxel` (`/Game/VoxelEngine/Test/Blueprints/BP_BlockPlacerPlayerController.VoxelWorld` _asbp_navigation_player_controller) (`/Game/VoxelEngine/Test/Blueprints/BP_BlockPlacerPlayerController.VoxelUnderCursor` _asbp_navigation_player_controller) 0))
          (if (`|EnumEquality` _returnvalue_2 "Executed")
            (`KismetSystemLibrary.PrintString` "Voxel destroyed")
            (else
              (`KismetSystemLibrary.PrintString` "Failed to destroy voxel" true true (struct :`R` 1.0 :`G` 0.009094 :`A` 1.0)))))))))

(fn `UserConstructionScript`)