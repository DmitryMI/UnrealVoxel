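; Test player controller for debugging voxel navigation, drawing the nav hierarchy under the cursor each tick.
; Releasing Space runs a debug path search between two fixed points on the VoxelWorld nav manager, storing visited nodes, their flags and the path.
; A looping timer replays the search one node box at a time, styled by flag, then draws the path in red and restarts.
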(event `CustomEvent`
  (`self.DrawVisitedNodes`))

(event `self.ReceiveBeginPlay`
  (`parent.ReceiveBeginPlay`)
  (`KismetSystemLibrary.K2_SetTimerDelegate` (delegate `CustomEvent`) (`self.DrawingPeriod`) true true))

(event `self.ReceiveTick`
  (params (DeltaSeconds :type "Float (single-precision)"))
  (`parent.ReceiveTick` DeltaSeconds)
  (if (`self.HasVoxelUnderCursor`)
    (`VoxelNavManagerComponent.DebugDrawNavHierarchy` (`VoxelWorld.GetVoxelNavManagerB` (`self.VoxelWorld`)) (`self.VoxelUnderCursor`))))

(event `Key|SpaceBar`
  (params (Key :type "Key Structure"))
  (:`Released`
    (bind (_outvisitednodes _outvisitednodesflags _returnvalue) (`VoxelNavManagerComponent.DebugFindPath` (`VoxelWorld.GetVoxelNavManagerB` (`self.VoxelWorld`)) (`KismetMathLibrary.MakeVector` 50.0 750.0 300.0) (`KismetMathLibrary.MakeVector` 750.0 50.0 200.0)))
    (set `self.VisitedNodes` _outvisitednodes)
    (set `self.VisitedNodesFlags` _outvisitednodesflags)
    (set `self.Path` _returnvalue)))

(fn `DrawPath`
  (for _array_element (`self.Path`)
    (`KismetSystemLibrary.DrawDebugBox` (`KismetMathLibrary.GetBoxCenter` _array_element) (/ (`KismetMathLibrary.GetBoxSize` _array_element) (2.0 2.0 2.0)) (struct :`R` 0.854167 :`B` 0.012173 :`A` 1.0) (struct) (* (`KismetArrayLibrary.Array_Length` (`self.VisitedNodes`)) (`self.DrawingPeriod`)) 3.0)))

(fn `DrawVisitedNodes`
  (bind _visualizationstep (`self.VisualizationStep`))
  (bind _output (`|GetArrayItem` (`self.VisitedNodes`) _visualizationstep))
  (bind _returnvalue (`KismetMathLibrary.GetBoxCenter` _output))
  (bind _returnvalue_2 (/ (`KismetMathLibrary.GetBoxSize` _output) (2.0 2.0 2.0)))
  (bind _returnvalue_3 (* (- (`KismetArrayLibrary.Array_Length` (`self.VisitedNodes`)) (`self.VisualizationStep`)) (`self.DrawingPeriod`)))
  (if (> (`KismetArrayLibrary.Array_Length` (`self.VisitedNodes`)) _visualizationstep)
    (if (`|GetArrayItem` (`self.VisitedNodesFlags`) _visualizationstep)
      (`KismetSystemLibrary.DrawDebugBox` _returnvalue _returnvalue_2 (struct :`G` 0.854167 :`B` 0.090583 :`A` 1.0) (struct) _returnvalue_3 2.0)
      (else
        (`KismetSystemLibrary.DrawDebugBox` _returnvalue _returnvalue_2 (struct :`G` 0.34375 :`B` 0.013908 :`A` 1.0) (struct) _returnvalue_3)))
    (set `self.VisualizationStep` (+ (`self.VisualizationStep`) 1))
    (if (not (> (`KismetArrayLibrary.Array_Length` (`self.VisitedNodes`)) (`self.VisualizationStep`)))
      (set `self.VisualizationStep` 0)
      (`self.DrawPath`))
    (else
      (set `self.VisualizationStep` 0))))

(fn `UserConstructionScript`
  (`parent.UserConstructionScript`))