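; BP_NavigationPawn is a player-controlled pawn in the VoxelEngine navigation test folder.
; Enhanced Input actions for forward, backward, right and left feed AddMovementInput along the actor's forward and right vectors, on both Triggered and Ongoing.
; The jump action adds world-up movement input instead of calling a jump.
; Tick and the construction script are empty.
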(event `self.ReceiveTick`
  (params (DeltaSeconds :type "Float (single-precision)")))

(event `EnhancedInput|/Game/VoxelEngine/Test/Input/IA_MoveForward`
  (params (ActionValue :type Boolean) (ElapsedSeconds :type "Float (double-precision)") (TriggeredSeconds :type "Float (double-precision)") (InputAction :type "InputAction Object Reference" :default "/Game/VoxelEngine/Test/Input/IA_MoveForward.IA_MoveForward"))
  (:`Triggered`
    (`self.AddMovementInput` (`self.GetActorForwardVector`) :!label _label))
  (:`Ongoing`
    (goto _label)))

(event `EnhancedInput|/Game/VoxelEngine/Test/Input/IA_MoveBackward`
  (params (ActionValue :type Boolean) (ElapsedSeconds :type "Float (double-precision)") (TriggeredSeconds :type "Float (double-precision)") (InputAction :type "InputAction Object Reference" :default "/Game/VoxelEngine/Test/Input/IA_MoveBackward.IA_MoveBackward"))
  (:`Triggered`
    (`self.AddMovementInput` (`self.GetActorForwardVector`) -1.0 :!label _label_2))
  (:`Ongoing`
    (goto _label_2)))

(event `EnhancedInput|/Game/VoxelEngine/Test/Input/IA_MoveRight`
  (params (ActionValue :type Boolean) (ElapsedSeconds :type "Float (double-precision)") (TriggeredSeconds :type "Float (double-precision)") (InputAction :type "InputAction Object Reference" :default "/Game/VoxelEngine/Test/Input/IA_MoveRight.IA_MoveRight"))
  (:`Triggered`
    (`self.AddMovementInput` (`self.GetActorRightVector`) :!label _label_3))
  (:`Ongoing`
    (goto _label_3)))

(event `EnhancedInput|/Game/VoxelEngine/Test/Input/IA_MoveLeft`
  (params (ActionValue :type Boolean) (ElapsedSeconds :type "Float (double-precision)") (TriggeredSeconds :type "Float (double-precision)") (InputAction :type "InputAction Object Reference" :default "/Game/VoxelEngine/Test/Input/IA_MoveLeft.IA_MoveLeft"))
  (:`Triggered`
    (`self.AddMovementInput` (`self.GetActorRightVector`) -1.0 :!label _label_4))
  (:`Ongoing`
    (goto _label_4)))

(event `EnhancedInput|/Game/VoxelEngine/Test/Input/IA_Jump`
  (params (ActionValue :type Boolean) (ElapsedSeconds :type "Float (double-precision)") (TriggeredSeconds :type "Float (double-precision)") (InputAction :type "InputAction Object Reference" :default "/Game/VoxelEngine/Test/Input/IA_Jump.IA_Jump"))
  (:`Triggered`
    (`self.AddMovementInput` (0.0 0.0 1.0))))

(fn `UserConstructionScript`)